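; AC-130 killstreak projectile that plays cosmetic explosion effects when its payload activates.
; PayloadActivated skips dedicated servers and projectiles with a valid predicted client counterpart, avoiding duplicate effects.
; Otherwise it plays a radial world camera shake, a pooled, randomly yawed particle explosion and a random sound with varied volume and pitch.
; The sound's validity check and playback roll separate random indices, so they can pick different entries.
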(event EventPayloadActivated
  (params (ImpactHitResult :type Hit%20Result%20Structure%20%28by%20ref%29))
  (bind _returnvalue (Math|Random|RandomFloatinRange 0.8 1.2))
  (bind _explosionsnd (Variables|Default|GetExplosionSnd))
  (bind _returnvalue_2 (Utilities|Array|LastIndex _explosionsnd))
  (bind _returnvalue_3 (Math|Random|RandomIntegerinRange 0 _returnvalue_2))
  (bind _output (Utilities|Array|Get(acopy) _explosionsnd _returnvalue_3))
  (if (not (or (Class|DFBaseProjectile|HasValidPredictedClientProjectile) (Networking|IsDedicatedServer))) ; Don't spawn explosion fx for this\nprojectile if a predicted one is\nassociated with it.
    (Utilities|FlowControl|Sequence
      (:then_0
        (Camera|PlayWorldCameraShake (Variables|Default|GetCameraShake) (Transformation|GetActorLocation) (Variables|Default|GetCameraShakeInnerRadius) (Variables|Default|GetCameraShakeOuterRadius) 1.0 true)
        (bind _explosionps (Variables|Default|GetExplosionPS)
          (:then
            (Effects|SpawnEmitteratLocation _explosionps (Transformation|GetActorLocation) (Math|Rotator|MakeRotator 0.0 0.0 (Math|Random|RandomFloatinRange 0.0 3.6e+02)) (Variables|Default|GetExplosionScale) true "AutoRelease"))
          (:else)))
      (:then_1
        (Utilities|IsValid _output
          (:Is%20Valid
            (Audio|PlaySoundatLocation _output (Transformation|GetActorLocation) "0, 0, 0" _returnvalue _returnvalue 0.0 0 0 0)))))))

(fn ConstructionScript)