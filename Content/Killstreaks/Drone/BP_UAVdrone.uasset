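; Possessable UAV drone killstreak that circles a server-spawned spline for a limited lifetime while the player aims, zooms and fires missiles from alternating pods.
; While a missile is live, a server camera trace steers its target point.
; A timer tags characters and vehicles with team custom-depth stencils and creates enemy outline widgets.
; Toggled thermal mode enables post-process and shows scaled screen-space outlines on enemies in line of sight.
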(event Custom|Fire
  (if (not (Variables|Default|GetIsFiring))
    (bind _returnvalue (Game|SpawnActorfromClass "/Killstreaks/Killstreaks/Drone/BP_Missle.BP_Missle_C" (Transformation|GetWorldTransform (select (Variables|Default|GetDroneLaunchSide) (Variables|Default|GetRightPod) (Variables|Default|GetLeftPod))) "AlwaysSpawn" 0 0))
    (bind _output_get (Variables|Default|SetMissleRef _returnvalue))
    (Variables|/Killstreaks/Killstreaks/Drone/BP_Missle.BP_Missle_C|SetParentDrone _output_get self)
    (Variables|Default|SetIsFiring true)
    (Variables|Default|SetDroneLaunchSide (not (Variables|Default|GetDroneLaunchSide)))))

(event Custom|MissleHit
  (Variables|Default|SetIsFiring false))

(event Custom|EndOfLife
  (Actor|DestroyActor))

(event Custom|RunOnLastClient
  (params (TargetClient :type HD%20Player%20Controller%20Object%20Reference))
  (if (== TargetClient (Game|GetPlayerController 0))
    (if (not (Networking|IsDedicatedServer))
      (CallFunction|CleanUp))))

(event Custom|Setup
  (CallFunction|SetupUI)
  (Variables|Default|SetNetPriority self 8.0)
  (Utilities|Time|SetTimerbyFunctionName 0 "IdentifyEnemies" 1.0 true)
  (bind _asbp_hdplayer_camera_manager_base (Utilities|Casting|CastToBP_HDPlayerCameraManagerBase (Game|GetPlayerCameraManager 0)))
  (Variables|Default|SetOriginalFOV (Variables|/Script/Engine.PlayerCameraManager|GetDefaultFOV _asbp_hdplayer_camera_manager_base))
  (Variables|Default|SetThermalMode false)
  (bind _ashdplayer_controller (Utilities|Casting|CastToHDPlayerController (Game|GetPlayerController 0)))
  (Variables|Default|SetCachedPlayerController _ashdplayer_controller))

(event EventBeginPlay
  (Networking|SwitchHasAuthority
    (:Authority
      (bind _returnvalue (Game|SpawnActorfromClass "/Killstreaks/Killstreaks/Drone/BP_DroneSpline.BP_DroneSpline_C" (Transformation|GetWorldTransform (Variables|Character|GetMesh)) "Undefined" 0 0))
      (Default|Setup _returnvalue self)
      (bind _output_get (Variables|Default|SetdroneSpline _returnvalue))
      (Default|CircleSplineMaker _output_get (Variables|/Killstreaks/Killstreaks/Drone/BP_DroneSpline.BP_DroneSpline_C|GetSpline _output_get) (Variables|Default|GetFlightRadius) 5)
      (CallFunction|UpdateRepPoints)
      (Utilities|Time|SetTimerbyEvent (delegate Custom|EndOfLife) (Variables|Default|GetDroneLifeTimeSec))
      (bind _alpha (Timeline|Timeline_0 Play)
        (:Update
          (Utilities|IsValid (Variables|Default|GetdroneSpline)
            (:Is%20Valid
              (Transformation|SetWorldLocationAndRotation (Variables|Character|GetMesh) (.location (Spline|GetTransformatDistanceAlongSpline (Variables|/Killstreaks/Killstreaks/Drone/BP_DroneSpline.BP_DroneSpline_C|GetSpline (Variables|Default|GetdroneSpline)) (Math|Float|Lerp 0.0 (Spline|GetSplineLength (Variables|/Killstreaks/Killstreaks/Drone/BP_DroneSpline.BP_DroneSpline_C|GetSpline (Variables|Default|GetdroneSpline))) _alpha) "World" false)) (Math|Rotator|MakeRotator (+ -2e+01 (.Roll (Math|Rotator|BreakRotator (.rotation (Spline|GetTransformatDistanceAlongSpline (Variables|/Killstreaks/Killstreaks/Drone/BP_DroneSpline.BP_DroneSpline_C|GetSpline (Variables|Default|GetdroneSpline)) (Math|Float|Lerp 0.0 (Spline|GetSplineLength (Variables|/Killstreaks/Killstreaks/Drone/BP_DroneSpline.BP_DroneSpline_C|GetSpline (Variables|Default|GetdroneSpline))) _alpha) "World" false))))) (.Pitch (Math|Rotator|BreakRotator (.rotation (Spline|GetTransformatDistanceAlongSpline (Variables|/Killstreaks/Killstreaks/Drone/BP_DroneSpline.BP_DroneSpline_C|GetSpline (Variables|Default|GetdroneSpline)) (Math|Float|Lerp 0.0 (Spline|GetSplineLength (Variables|/Killstreaks/Killstreaks/Drone/BP_DroneSpline.BP_DroneSpline_C|GetSpline (Variables|Default|GetdroneSpline))) _alpha) "World" false)))) (.Yaw (Math|Rotator|BreakRotator (.rotation (Spline|GetTransformatDistanceAlongSpline (Variables|/Killstreaks/Killstreaks/Drone/BP_DroneSpline.BP_DroneSpline_C|GetSpline (Variables|Default|GetdroneSpline)) (Math|Float|Lerp 0.0 (Spline|GetSplineLength (Variables|/Killstreaks/Killstreaks/Drone/BP_DroneSpline.BP_DroneSpline_C|GetSpline (Variables|Default|GetdroneSpline))) _alpha) "World" false))))) false false))))))))

(event EventPossessed
  (params (NewController :type Controller%20Object%20Reference))
  (bind _ashdplayer_controller (Utilities|Casting|CastToHDPlayerController NewController))
  (Variables|Default|SetCachedPlayerController _ashdplayer_controller)
  (CallFunction|Setup))

(event EventUnpossessed
  (params (OldController :type Controller%20Object%20Reference))
  (CallFunction|RunonLastClient (Variables|Default|GetCachedPlayerController))
  (Development|PrintString "UNPOSSESSED"))

(event EventTick
  (params (DeltaSeconds :type Float%20%28single-precision%29))
  (Utilities|FlowControl|Sequence
    (:then_0
      (if (Pawn|IsLocallyControlled)
        (CallFunction|TickThermal)))
    (:then_1
      (Networking|SwitchHasAuthority
        (:Authority
          (if (Variables|Default|GetIsFiring)
            (CallFunction|UpdateTargetLocation)))))))

(event Input|MouseEvents|MouseX
  (params (AxisValue :type Float%20%28single-precision%29))
  (Pawn|Input|AddControllerYawInput AxisValue))

(event Input|MouseEvents|MouseY
  (params (AxisValue :type Float%20%28single-precision%29))
  (bind _returnvalue (* -1 AxisValue))
  (bind _returnvalue_2 (Pawn|GetControlRotation :!class /Script/Engine.Pawn))
  (Pawn|Input|AddControllerPitchInput _returnvalue)
  (Pawn|SetControlRotation (Variables|Default|GetCachedPlayerController) (Math|Rotator|MakeRotator 0.0 (Class|KismetMathLibrary|ClampAxis (Math|Float|ClampAngle (+ _returnvalue (.pitch _returnvalue_2)) -9e+01 1e+01)) (.yaw _returnvalue_2))))

(event Input|KeyboardEvents|Q
  (params (Key :type Key%20Structure))
  (:Pressed
    (bind _asbp_hdplayer_camera_manager_base (Utilities|Casting|CastToBP_HDPlayerCameraManagerBase (Game|GetPlayerCameraManager 0)))
    (if (Variables|Default|GetzoomToggle)
      (Variables|/Script/Engine.PlayerCameraManager|SetDefaultFOV _asbp_hdplayer_camera_manager_base 7e+01)
      (Variables|Default|SetzoomToggle false)
      (else
        (Variables|/Script/Engine.PlayerCameraManager|SetDefaultFOV _asbp_hdplayer_camera_manager_base 2e+01)
        (Variables|Default|SetzoomToggle true)))))

(event Input|MouseEvents|MiddleMouseButton
  (params (Key :type Key%20Structure))
  (:Pressed
    (CallFunction|Fire)))

(event Input|KeyboardEvents|T
  (params (Key :type Key%20Structure))
  (bind _postprocess (Variables|Default|GetPostProcess))
  (:Pressed
    (Utilities|FlowControl|FlipFlop
      (:A
        (Variables|/Script/Engine.PostProcessComponent|SetbEnabled _postprocess true)
        (Variables|Default|SetThermalMode true))
      (:B
        (Variables|/Script/Engine.PostProcessComponent|SetbEnabled _postprocess false)
        (Variables|Default|SetThermalMode false)
        (bind _values (Utilities|Map|Values (Variables|Default|GetEnemyPlayers)))
        (for _array_element _values
          (Widget|SetVisibility _array_element "Hidden"))))))

(fn ConstructionScript)

(fn UpdateRepPoints
  (bind _helperarray (LocalVariables|GethelperArray))
  (bind _dronespline (Variables|Default|GetdroneSpline))
  (bind _spline (Variables|/Killstreaks/Killstreaks/Drone/BP_DroneSpline.BP_DroneSpline_C|GetSpline _dronespline))
  (Utilities|Array|Clear _helperarray)
  (for _index (range 0 (- (Spline|GetNumberOfSplinePoints _spline) 1))
    (Utilities|Array|AppendArray _helperarray (Utilities|Array|MakeArray (Utilities|Struct|MakeReplicatedSplinePoints (Spline|GetLocationatSplinePoint _spline _index "World") (Spline|GetTangentatSplinePoint _spline _index "World")))))
  (Variables|/Killstreaks/Killstreaks/Drone/BP_DroneSpline.BP_DroneSpline_C|SetDroneSplinePoints (Variables|Default|GetdroneSpline) _helperarray))

(fn OnRepDroneSplinePoints
  (bind _dronespline (Variables|Default|GetdroneSpline))
  (bind _spline (Variables|/Killstreaks/Killstreaks/Drone/BP_DroneSpline.BP_DroneSpline_C|GetSpline _dronespline))
  (Utilities|IsValid (Variables|Default|GetdroneSpline)
    (:Is%20Valid
      (Spline|ClearSplinePoints _spline false)
      (for (_array_element _array_index) 0
        (Spline|AddSplinePoint _spline (.Location (Utilities|Struct|BreakReplicatedSplinePoints _array_element)) "World" false)
        (Spline|SetTangentatSplinePoint _spline _array_index (.Tangent (Utilities|Struct|BreakReplicatedSplinePoints _array_element)) "World" false))
      (Spline|UpdateSpline _spline)
      (return))))

(fn CleanUp
  (Variables|Default|SetNetPriority self 3.0)
  (Variables|/Script/Engine.PostProcessComponent|SetbEnabled (Variables|Default|GetPostProcess) false)
  (Utilities|Time|ClearTimerbyFunctionName 0 "IdentifyEnemies")
  (CallFunction|CleanUpUI)
  (bind _asbp_hdplayer_camera_manager_base (Utilities|Casting|CastToBP_HDPlayerCameraManagerBase (Game|GetPlayerCameraManager 0)))
  (Variables|/Script/Engine.PlayerCameraManager|SetDefaultFOV _asbp_hdplayer_camera_manager_base (Variables|Default|GetOriginalFOV)))

(fn IdentifyEnemies
  (Utilities|FlowControl|Sequence
    (:then_0
      (bind _outactors (Actor|GetAllActorsOfClass "/HDCore/Core/BP_HDPlayerCharacterBase.BP_HDPlayerCharacterBase_C"))
      (for _array_element _outactors
        (if (not (Utilities|Map|Contains (Variables|Default|GetEnemyPlayers) _array_element))
          (Rendering|SetRenderCustomDepth (Variables|/Script/Engine.Character|GetMesh _array_element) true)
          (if (== (Class|DFBlueprintFunctions|GetTeamNum _array_element) (Class|DFBlueprintFunctions|GetTeamNum self))
            (Rendering|SetCustomDepthStencilValue (Variables|/Script/Engine.Character|GetMesh _array_element) 2)
            (else
              (Rendering|SetCustomDepthStencilValue (Variables|/Script/Engine.Character|GetMesh _array_element) 1)
              (bind _returnvalue (UserInterface|CreateWidget "/Killstreaks/Killstreaks/Drone/DroneUI/EnemyOutline.EnemyOutline_C"))
              (Utilities|Map|Add (Variables|Default|GetEnemyPlayers) _array_element _returnvalue)
              (UserInterface|Viewport|AddtoViewport _returnvalue 0)
              (Widget|SetVisibility _returnvalue "Hidden")
              (EventDispatchers|BindEventtoOnCharacterDeath _array_element (EventDispatchers|CreateEvent :!event RemoveDestroyedPlayers)))))))
    (:then_1
      (bind _outactors_2 (Actor|GetAllActorsOfClass "/Script/HDMain.HDBaseVehicle"))
      (for _array_element_2 _outactors_2
        (if (not (Utilities|Map|Contains (Variables|Default|GetEnemyVehicles) _array_element_2))
          (Rendering|SetRenderCustomDepth (Variables|/Script/HDMain.HDBaseVehicle|GetMesh _array_element_2) true)
          (if (== (Class|DFBlueprintFunctions|GetTeamNum _array_element_2) (Class|DFBlueprintFunctions|GetTeamNum self))
            (Rendering|SetCustomDepthStencilValue (Variables|/Script/HDMain.HDBaseVehicle|GetMesh _array_element_2) 2)
            (else
              (Rendering|SetCustomDepthStencilValue (Variables|/Script/HDMain.HDBaseVehicle|GetMesh _array_element_2) 1)
              (bind _returnvalue_2 (UserInterface|CreateWidget "/Killstreaks/Killstreaks/Drone/DroneUI/EnemyOutline.EnemyOutline_C"))
              (Utilities|Map|Add (Variables|Default|GetEnemyVehicles) _array_element_2 _returnvalue_2)
              (UserInterface|Viewport|AddtoViewport _returnvalue_2 0)
              (Widget|SetVisibility _returnvalue_2 "Hidden")
              (EventDispatchers|BindEventtoOnVehicleDestroyed _array_element_2 (EventDispatchers|CreateEvent :!event BPUAVdroneAutoGenFunc))
              (Development|PrintString "AddingVehicle"))))))))

(fn SetupUI
  (bind _asbp_hdhudbase (Utilities|Casting|CastToBP_HDHUDBase (HUD|GetHUD (Game|GetPlayerController 0))))
  (Variables|/HDCore/Core/BP_HDHUDBase.BP_HDHUDBase_C|SetVehicleHUDContainerUWClass _asbp_hdhudbase "/Killstreaks/Killstreaks/Drone/DroneUI/DroneCrossHair.DroneCrossHair_C")
  (Default|SetIsVehicleHUDWidgetActive _asbp_hdhudbase true)
  (bind _asdrone_cross_hair (Utilities|Casting|CastToDroneCrossHair (Default|GetValidVehicleHUDContainer _asbp_hdhudbase)))
  (Variables|Default|SetHUDCrosshair _asdrone_cross_hair))

(fn CleanUpUI
  (bind _enemyplayers (Variables|Default|GetEnemyPlayers))
  (bind _asbp_hdhudbase (Utilities|Casting|CastToBP_HDHUDBase (HUD|GetHUD (Game|GetPlayerController 0))))
  (Default|SetIsVehicleHUDWidgetActive _asbp_hdhudbase false)
  (Default|DestroyWidget (Variables|Default|GetHUDCrosshair))
  (bind _values (Utilities|Map|Values _enemyplayers))
  (for _array_element _values
    (Widget|RemovefromParent _array_element)
    (Utilities|Map|Clear _enemyplayers)))

(fn RemoveDestroyedPlayers
  (params (VictimPawn :type Pawn%20Object%20Reference) (VictimController :type Controller%20Object%20Reference) (KillingDamage :type Float%20%28single-precision%29) (DamageEvent :type Damage%20Event%20Structure%20%28by%20ref%29) (InstigatingPawn :type Pawn%20Object%20Reference) (DamageCauser :type Actor%20Object%20Reference))
  (bind _asbp_hdplayer_character_base (Utilities|Casting|CastToBP_HDPlayerCharacterBase VictimPawn)
    (:then
      (if (.ReturnValue (Utilities|Map|Find (Variables|Default|GetEnemyPlayers) _asbp_hdplayer_character_base))
        (Widget|RemovefromParent (.Value (Utilities|Map|Find (Variables|Default|GetEnemyPlayers) _asbp_hdplayer_character_base)))
        (return)))
    (:CastFailed
      (Development|PrintString "DID NOT FIND CHARACTER"))))

(fn TickThermal
  (bind _cachedplayercontroller (Variables|Default|GetCachedPlayerController))
  (bind _enemyplayers (Variables|Default|GetEnemyPlayers))
  (bind _cachedplayercontroller_2 (Variables|Default|GetCachedPlayerController))
  (bind _enemyvehicles (Variables|Default|GetEnemyVehicles))
  (bind (_sizex _sizey) (HUD|GetViewportSize _cachedplayercontroller_2))
  (bind (_sizex_2 _sizey_2) (HUD|GetViewportSize _cachedplayercontroller))
  (if (Variables|Default|GetThermalMode)
    (Utilities|FlowControl|Sequence
      (:then_0
        (bind _keys (Utilities|Map|Keys _enemyplayers))
        (for _array_element _keys
          (Utilities|IsValid _array_element
            (:Is%20Valid
              (if (.ReturnValue (Class|GameplayStatics|ProjectWorldtoScreen _cachedplayercontroller_2 (Class|SkeletalMeshComponent|GetSkeletalCenterOfMass (Variables|/Script/Engine.Character|GetMesh _array_element)) false))
                (bind _returnvalue (Collision|LineTraceByChannel (Transformation|GetWorldLocation (Variables|Default|GetDroneCamera)) (Class|SkeletalMeshComponent|GetSkeletalCenterOfMass (Variables|/Script/Engine.Character|GetMesh _array_element)) "TraceTypeQuery1" true (Utilities|Array|MakeArray _array_element) "None"))
                (if _returnvalue
                  (Widget|SetVisibility (.Value (Utilities|Map|Find _enemyplayers _array_element)) "Hidden" :!label _label)
                  (else
                    (Class|UserWidget|SetPositioninViewport (.Value (Utilities|Map|Find _enemyplayers _array_element)) (- (.ScreenPosition (Class|GameplayStatics|ProjectWorldtoScreen _cachedplayercontroller_2 (Class|SkeletalMeshComponent|GetSkeletalCenterOfMass (Variables|/Script/Engine.Character|GetMesh _array_element)) false)) (|OutlineCenterAdjust (Math|Conversions|ToFloat(Integer) _sizex) (Math|Conversions|ToFloat(Integer) _sizey))) true)
                    (Widget|SetVisibility (.Value (Utilities|Map|Find _enemyplayers _array_element)) "Visible")
                    (Widget|Transform|SetRenderScale (.Value (Utilities|Map|Find _enemyplayers _array_element)) (Math|Vector2D|MakeVector2D (Math|Float|Clamp(Float) (+ (/ (Math|Float|Absolute(Float) (Math|Vector|Distance2D(Vector) (|HalfPlayerThicknessOnScreen (Variables|/Script/Engine.Character|GetMesh _array_element)) (.ScreenPosition (Class|GameplayStatics|ProjectWorldtoScreen _cachedplayercontroller_2 (Class|SkeletalMeshComponent|GetSkeletalCenterOfMass (Variables|/Script/Engine.Character|GetMesh _array_element)) false)))) 25.0) 0.25) 0.5 2e+02) (Math|Float|Clamp(Float) (+ (/ (Math|Float|Absolute(Float) (Math|Vector|Distance2D(Vector) (|HalfPlayerThicknessOnScreen (Variables|/Script/Engine.Character|GetMesh _array_element)) (.ScreenPosition (Class|GameplayStatics|ProjectWorldtoScreen _cachedplayercontroller_2 (Class|SkeletalMeshComponent|GetSkeletalCenterOfMass (Variables|/Script/Engine.Character|GetMesh _array_element)) false)))) 25.0) 0.25) 0.5 2e+02)))))
                (else
                  (goto _label)))))))
      (:then_1
        (bind _keys_2 (Utilities|Map|Keys _enemyvehicles))
        (for _array_element_2 _keys_2
          (Utilities|IsValid _array_element_2
            (:Is%20Valid
              (if (.ReturnValue (Class|GameplayStatics|ProjectWorldtoScreen _cachedplayercontroller (Class|SkeletalMeshComponent|GetSkeletalCenterOfMass (Variables|/Script/HDMain.HDBaseVehicle|GetMesh _array_element_2)) false))
                (bind _returnvalue_2 (Collision|LineTraceByChannel (Transformation|GetWorldLocation (Variables|Default|GetDroneCamera)) (Class|SkeletalMeshComponent|GetSkeletalCenterOfMass (Variables|/Script/HDMain.HDBaseVehicle|GetMesh _array_element_2)) "TraceTypeQuery1" true (Utilities|Array|MakeArray _array_element_2) "None"))
                (if _returnvalue_2
                  (Widget|SetVisibility (.Value (Utilities|Map|Find _enemyvehicles _array_element_2)) "Hidden" :!label _label_2)
                  (else
                    (Class|UserWidget|SetPositioninViewport (.Value (Utilities|Map|Find _enemyvehicles _array_element_2)) (- (.ScreenPosition (Class|GameplayStatics|ProjectWorldtoScreen _cachedplayercontroller (Class|SkeletalMeshComponent|GetSkeletalCenterOfMass (Variables|/Script/HDMain.HDBaseVehicle|GetMesh _array_element_2)) false)) (|OutlineCenterAdjust_2 (Math|Conversions|ToFloat(Integer) _sizex_2) (Math|Conversions|ToFloat(Integer) _sizey_2))) true)
                    (Widget|SetVisibility (.Value (Utilities|Map|Find _enemyvehicles _array_element_2)) "Visible")
                    (Widget|Transform|SetRenderScale (.Value (Utilities|Map|Find _enemyvehicles _array_element_2)) (Math|Vector2D|MakeVector2D (Math|Float|Clamp(Float) (+ (/ (Math|Float|Absolute(Float) (Math|Vector|Distance2D(Vector) (|HalfPlayerThicknessOnScreen_2 (Variables|/Script/HDMain.HDBaseVehicle|GetMesh _array_element_2)) (.ScreenPosition (Class|GameplayStatics|ProjectWorldtoScreen _cachedplayercontroller (Class|SkeletalMeshComponent|GetSkeletalCenterOfMass (Variables|/Script/HDMain.HDBaseVehicle|GetMesh _array_element_2)) false)))) 25.0) 0.25) 0.5 2e+02) (Math|Float|Clamp(Float) (+ (/ (Math|Float|Absolute(Float) (Math|Vector|Distance2D(Vector) (|HalfPlayerThicknessOnScreen_2 (Variables|/Script/HDMain.HDBaseVehicle|GetMesh _array_element_2)) (.ScreenPosition (Class|GameplayStatics|ProjectWorldtoScreen _cachedplayercontroller (Class|SkeletalMeshComponent|GetSkeletalCenterOfMass (Variables|/Script/HDMain.HDBaseVehicle|GetMesh _array_element_2)) false)))) 25.0) 0.25) 0.5 2e+02)))))
                (else
                  (goto _label_2))))))))))

(fn BPUAVdroneAutoGenFunc
  (params (Vehicle :type HD%20Base%20Vehicle%20Object%20Reference))
  (bind _enemyvehicles (Variables|Default|GetEnemyVehicles))
  (bind (_value _returnvalue) (Utilities|Map|Find _enemyvehicles Vehicle))
  (Utilities|IsValid Vehicle
    (:Is%20Valid
      (if _returnvalue
        (Widget|RemovefromParent _value)))
    (:Is%20Not%20Valid
      (Development|PrintString "DID NOT FIND CHARACTER"))))

(fn UpdateTargetLocation
  (bind _dronecamera (Variables|Default|GetDroneCamera))
  (bind _returnvalue (Transformation|GetWorldLocation _dronecamera))
  (bind (_outhit _returnvalue_2) (Collision|LineTraceByChannel _returnvalue (+ _returnvalue (* (Math|Vector|GetForwardVector (Pawn|GetControlRotation :!class /Script/Engine.Pawn)) 7e+04)) "TraceTypeQuery1" false 0 "None"))
  (if _returnvalue_2
    (Variables|/Killstreaks/Killstreaks/Drone/BP_Missle.BP_Missle_C|SetTargetLocation (Variables|Default|GetMissleRef) (.ImpactPoint (Collision|BreakHitResult _outhit)))))