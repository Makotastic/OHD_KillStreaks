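; Spline actor for a drone that holds a path, built by default as a flat circle around its origin.
; The construction script places evenly spaced points with tangents scaled by a tangent-based arc formula to round the curve; CircleSplineMaker duplicates this logic.
; A RepNotify on DroneSplinePoints rebuilds the spline from world-space locations and tangents.
; Setup binds to the parent drone's destruction event, with DestroySelf available to remove the actor.
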(event EventBeginPlay)

(fn ConstructionScript
  (CallFunction|CunstructionHelper (Variables|Default|GetSpline) 2e+03 5))

(fn CunstructionHelper
  (params (splineComp :type Spline%20Component%20Object%20Reference) (Radius :type Float%20%28single-precision%29) (segments :type Integer))
  (bind _returnvalue (- segments 1))
  (Spline|ClearSplinePoints splineComp false)
  (if (> segments 0)
    (for _index (range 0 _returnvalue)
      (Spline|AddSplinePoint splineComp (Math|Vector|MakeVector (* (Math|Trig|Sin(Degrees) (Math|Float|MapRangeClamped (Math|Conversions|ToFloat(Integer) _index) 0.0 (Math|Conversions|ToFloat(Integer) _returnvalue) 0.0 (Math|Conversions|ToFloat(Integer) (|(360-(360/vSegments)) segments)))) Radius) (* (Math|Trig|Cos(Degrees) (Math|Float|MapRangeClamped (Math|Conversions|ToFloat(Integer) _index) 0.0 (Math|Conversions|ToFloat(Integer) _returnvalue) 0.0 (Math|Conversions|ToFloat(Integer) (|(360-(360/vSegments)) segments)))) Radius) 0.0) "Local" false)
      (Spline|SetTangentatSplinePoint splineComp _index (* (Math|Vector|GetRightVector (Math|Rotator|FindLookatRotation (Math|Vector|MakeVector (* (Math|Trig|Sin(Degrees) (Math|Float|MapRangeClamped (Math|Conversions|ToFloat(Integer) _index) 0.0 (Math|Conversions|ToFloat(Integer) _returnvalue) 0.0 (Math|Conversions|ToFloat(Integer) (|(360-(360/vSegments)) segments)))) Radius) (* (Math|Trig|Cos(Degrees) (Math|Float|MapRangeClamped (Math|Conversions|ToFloat(Integer) _index) 0.0 (Math|Conversions|ToFloat(Integer) _returnvalue) 0.0 (Math|Conversions|ToFloat(Integer) (|(360-(360/vSegments)) segments)))) Radius) 0.0) (Math|Vector|MakeVector 0.0 0.0 0.0))) (* Radius (|(4*(tan(((D2R((360/vSegments)))/4)))) segments))) "Local" false)))
  (Spline|UpdateSpline splineComp)
  (return))

(fn CircleSplineMaker
  (params (SplineComp :type Spline%20Component%20Object%20Reference) (Radius :type Float%20%28single-precision%29) (Nodes :type Integer))
  (bind _returnvalue (- Nodes 1))
  (Spline|ClearSplinePoints SplineComp false)
  (if (> Nodes 0)
    (for _index (range 0 _returnvalue)
      (Spline|AddSplinePoint SplineComp (Math|Vector|MakeVector (* (Math|Trig|Sin(Degrees) (Math|Float|MapRangeClamped (Math|Conversions|ToFloat(Integer) _index) 0.0 (Math|Conversions|ToFloat(Integer) _returnvalue) 0.0 (Math|Conversions|ToFloat(Integer) (|(360-(360/vSegments)) Nodes)))) Radius) (* (Math|Trig|Cos(Degrees) (Math|Float|MapRangeClamped (Math|Conversions|ToFloat(Integer) _index) 0.0 (Math|Conversions|ToFloat(Integer) _returnvalue) 0.0 (Math|Conversions|ToFloat(Integer) (|(360-(360/vSegments)) Nodes)))) Radius) 0.0) "Local" false)
      (Spline|SetTangentatSplinePoint SplineComp _index (* (Math|Vector|GetRightVector (Math|Rotator|FindLookatRotation (Math|Vector|MakeVector (* (Math|Trig|Sin(Degrees) (Math|Float|MapRangeClamped (Math|Conversions|ToFloat(Integer) _index) 0.0 (Math|Conversions|ToFloat(Integer) _returnvalue) 0.0 (Math|Conversions|ToFloat(Integer) (|(360-(360/vSegments)) Nodes)))) Radius) (* (Math|Trig|Cos(Degrees) (Math|Float|MapRangeClamped (Math|Conversions|ToFloat(Integer) _index) 0.0 (Math|Conversions|ToFloat(Integer) _returnvalue) 0.0 (Math|Conversions|ToFloat(Integer) (|(360-(360/vSegments)) Nodes)))) Radius) 0.0) (Math|Vector|MakeVector 0.0 0.0 0.0))) (* Radius (|(4*(tan(((D2R((360/vSegments)))/4)))) Nodes))) "Local" false)))
  (Spline|UpdateSpline SplineComp)
  (return))

(fn OnRepDroneSplinePoints
  (bind _spline (Variables|Default|GetSpline))
  (Spline|ClearSplinePoints _spline false)
  (for (_array_element _array_index) (Variables|Default|GetDroneSplinePoints)
    (Spline|AddSplinePoint _spline (.Location (Utilities|Struct|BreakReplicatedSplinePoints _array_element)) "World" false)
    (Spline|SetTangentatSplinePoint _spline _array_index (.Tangent (Utilities|Struct|BreakReplicatedSplinePoints _array_element)) "World" false))
  (Spline|UpdateSpline _spline)
  (return))

(fn Setup
  (params (ParentDrone :type BP%20UA%20Vdrone%20Object%20Reference))
  (Game|BindEventtoOnDestroyed ParentDrone (EventDispatchers|CreateEvent :!event DestroySelf)))

(fn DestroySelf
  (params (DestroyedActor :type Actor%20Object%20Reference))
  (Actor|DestroyActor))