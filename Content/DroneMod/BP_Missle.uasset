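; Guided missile fired by a parent drone that steers toward TargetLocation and explodes on impact.
; Each server tick rebuilds a two-point spline to the target, tangent to the rocket's heading, then sweeps along it.
; A huge tangent during brief launch arming keeps flyout straight.
; Blocking hits other than the drone deal radial damage sparing same-team characters, play effects and destroy it; impact or lifetime timeout notifies the drone.
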(event Custom|MissleExplosion
  (params (Location :type Vector))
  (Effects|SpawnEmitteratLocation "/IHaveNoIdea/DroneMod/OHD_STUFF/PS_Rocket_Explosion.PS_Rocket_Explosion" Location "0, 0, 0" "3.000000,3.000000,3.000000")
  (Audio|PlaySoundatLocation "/IHaveNoIdea/DroneMod/OHD_STUFF/A_Rocket_Explosion.A_Rocket_Explosion" Location "0, 0, 0" 1.5 1.0 0.0 0 0 0))

(event EventBeginPlay
  (Utilities|FlowControl|Delay 0.1)
  (Variables|Default|SetFlyout/Arming false)
  (Utilities|FlowControl|Delay 15.0)
  (Default|MissleHit (Variables|Default|GetParentDrone))
  (Actor|DestroyActor))

(event EventTick
  (params (DeltaSeconds :type Float%20%28single-precision%29))
  (bind _spline (Variables|Default|GetSpline))
  (bind _velocity (Variables|Default|GetVelocity))
  (bind _returnvalue (* _velocity DeltaSeconds))
  (bind _returnvalue_2 (Spline|GetTransformatDistanceAlongSpline _spline _returnvalue "World" false))
  (if (Ability|HasAuthority)
    (CallFunction|UpdateSpline)
    (bind _sweephitresult (Transformation|SetWorldLocationAndRotation (Variables|Default|GetRocket) (.location _returnvalue_2) (.rotation _returnvalue_2) true false))
    (CallFunction|HandleCollisionApplyDamge _sweephitresult)))

(fn ConstructionScript)

(fn UpdateSpline
  (bind _spline (Variables|Default|GetSpline))
  (Spline|ClearSplinePoints _spline false)
  (Spline|AddSplinePoint _spline (Transformation|GetWorldLocation (Variables|Default|GetRocket)) "World" false)
  (Spline|AddSplinePoint _spline (Variables|Default|GetTargetLocation) "World" false)
  (if (Variables|Default|GetFlyout/Arming)
    (Spline|SetTangentatSplinePoint _spline 0 (* (Math|Vector|GetForwardVector (Transformation|GetWorldRotation (Variables|Default|GetRocket))) 999999995904.0) "World" false)
    (Spline|UpdateSpline _spline)
    (else
      (Spline|SetTangentatSplinePoint _spline 0 (* (Math|Vector|GetForwardVector (Transformation|GetWorldRotation (Variables|Default|GetRocket))) (Variables|Default|GetVelocity)) "World" false)
      (Spline|UpdateSpline _spline))))

(fn HandleCollisionApplyDamge
  (params (Hit :type Hit%20Result%20Structure%20%28by%20ref%29))
  (bind (_bblockinghit _binitialoverlap _time _distance _location _impactpoint _normal _impactnormal _physmat _hitactor) (Collision|BreakHitResult Hit))
  (bind _parentdrone (Variables|Default|GetParentDrone))
  (if (and _bblockinghit (not (== _hitactor (Variables|Default|GetParentDrone))))
    (Utilities|IsValid _parentdrone
      (:Is%20Valid
        (Default|MissleHit _parentdrone)
        (bind _teammates (|IdentifiyTeammates)
          (:Completed
            (Class|GameplayStatics|ApplyRadialDamagewithFalloff 1e+04 0.0 _location 7e+02 1.5e+03 1.0 0 _teammates _parentdrone (Pawn|GetController _parentdrone) "ECC_GameTraceChannel1")
            (CallFunction|MissleExplosion _location)
            (Actor|DestroyActor)))))))